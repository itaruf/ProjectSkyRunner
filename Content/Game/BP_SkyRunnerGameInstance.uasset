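; BP_SkyRunnerGameInstance is the game instance that owns the lifetime of game-wide services, currently the inventory service.
; On Init it creates the inventory service, stores it, and, if valid, initializes it and registers it under the name "Inventory".
; On Shutdown it shuts down the inventory service if valid, then clears all registered services.
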(fn `Init`
  (locals (InventoryService :type "InventoryService Object Reference"))
  (bind _returnvalue (`InventoryService.CreateInventoryService` self))
  (bind _output_get (set `local.InventoryService` _returnvalue))
  (`/Engine/EditorBlueprintResources/StandardMacros.IsValid` _output_get
    (:`Is Valid`
      (`GameServiceInterface.InitializeService` (`local.InventoryService`))
      (`GameServiceLocator.RegisterService` "Inventory" (`local.InventoryService`)))))

(fn `Shutdown`
  (locals (InventoryService :type "InventoryService Object Reference"))
  (`|ExecutionSequence`
    (:`then_0`
      (bind _output_get (set `local.InventoryService` (`GameServiceLocator.GetInventoryService`)))
      (`/Engine/EditorBlueprintResources/StandardMacros.IsValid` _output_get
        (:`Is Valid`
          (`GameServiceInterface.ShutdownService` (`local.InventoryService`)))))
    (:`then_1`
      (`GameServiceLocator.ClearServices`))))